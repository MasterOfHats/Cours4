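; Player controller that routes movement, jump and camera input to the player pawn through message calls, along with a per-frame tick.
; A ControlType state gates input: Movement passes everything, Cam Only passes just camera axes, and Menu Opened blocks both.
; Debug keys toggle the control type, print a pawn message result, or save the pawn and static mesh actor positions to the default slot.
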(event `Key|Y`
  (params (Key :type "Key Structure"))
  (:`Pressed`
    (bind _output (message `/Game/Cours3/Core/BPI_Inputable.FunctionExample` (`GameplayStatics.GetPlayerPawn` 0)))
    (`KismetSystemLibrary.PrintString` (`KismetStringLibrary.Conv_BoolToString` _output))))

(event `self.ReceiveBeginPlay`
  (`self.SetActorTickEnabled` true))

(event `self.ReceiveTick`
  (params (DeltaSeconds :type "Float (single-precision)"))
  (switch `/Game/Cours3/Core/EControlType` (`self.ControlType`)
    (:`NewEnumerator0`
      _)
    (:`NewEnumerator1`
      _)
    (:`NewEnumerator2`
      _))
  (message `/Game/Cours3/Core/BPI_Inputable.ReceiveInputTick` (`GameplayStatics.GetPlayerPawn` 0) (`GameplayStatics.GetWorldDeltaSeconds`)))

(event `Key|C`
  (params (Key :type "Key Structure"))
  ;[1 1 1] Debug exemple
  (:`Pressed`
    (`/Engine/EditorBlueprintResources/StandardMacros.FlipFlop`
      (:`A`
        (set `self.ControlType` "NewEnumerator1"))
      (:`B`
        (set `self.ControlType` "NewEnumerator0")))))

(event `InputAction|InputJump`
  (params (Key :type "Key Structure"))
  (:`Pressed`
    (switch `/Game/Cours3/Core/EControlType` (`self.ControlType`)
      (:`NewEnumerator0`
        (message `/Game/Cours3/Core/BPI_Inputable.ReceiveInputJump` (`GameplayStatics.GetPlayerPawn` 0))))))

(event `Key|O`
  (params (Key :type "Key Structure"))
  ;[1 1 1] Debug exemple
  (:`Pressed`
    (bind _returnvalue (`self.SaveGame`))
    (if _returnvalue
      (`KismetSystemLibrary.PrintString` "SaveSuccesful"))))

(event `InputAxis|MoveForward`
  (params (AxisValue :type "Float (single-precision)"))
  (switch `/Game/Cours3/Core/EControlType` (`self.ControlType`)
    (:`NewEnumerator0`
      (message `/Game/Cours3/Core/BPI_Inputable.ReceiveAxisForward` (`GameplayStatics.GetPlayerPawn` 0) AxisValue))))

(event `InputAxis|MoveRight`
  (params (AxisValue :type "Float (single-precision)"))
  (switch `/Game/Cours3/Core/EControlType` (`self.ControlType`)
    (:`NewEnumerator0`
      (message `/Game/Cours3/Core/BPI_Inputable.ReceiveAxisRight` (`GameplayStatics.GetPlayerPawn` 0) AxisValue))))

(event `InputAxis|CameraUp`
  (params (AxisValue :type "Float (single-precision)"))
  (switch `/Game/Cours3/Core/EControlType` (`self.ControlType`)
    (:`NewEnumerator0`
      _)
    (:`NewEnumerator1`
      _))
  (message `/Game/Cours3/Core/BPI_Inputable.ReceiveCameraUp` (`GameplayStatics.GetPlayerPawn` 0) AxisValue))

(event `InputAxis|CameraRight`
  (params (AxisValue :type "Float (single-precision)"))
  (switch `/Game/Cours3/Core/EControlType` (`self.ControlType`)
    (:`NewEnumerator0`
      _)
    (:`NewEnumerator1`
      _))
  (message `/Game/Cours3/Core/BPI_Inputable.ReceiveCameraRight` (`GameplayStatics.GetPlayerPawn` 0) AxisValue))

(fn `SaveGame`
  (returns (ReturnValue :type Boolean))
  (locals (LocalSaveGame :type "/Game/Cours3/Core/SaveLoadSystem/BP_MainSaveGame Object Reference"))
  (`|ExecutionSequence`
    (:`then_0`
      (bind _returnvalue (`GameplayStatics.CreateSaveGameObject` "/Game/Cours3/Core/SaveLoadSystem/BP_MainSaveGame.BP_MainSaveGame_C"))
      (set `local.LocalSaveGame` _returnvalue)
      (set `/Game/Cours3/Core/SaveLoadSystem/BP_MainSaveGame.PlayerPosition` (`self.K2_GetActorLocation` (`GameplayStatics.GetPlayerPawn` 0)) (`local.LocalSaveGame`))
      (bind _outactors (`GameplayStatics.GetAllActorsOfClass` "/Script/Engine.StaticMeshActor"))
      (for (_array_element _array_index) _outactors
        (`KismetArrayLibrary.Array_Set` (`/Game/Cours3/Core/SaveLoadSystem/BP_MainSaveGame.ActorPositions` (`local.LocalSaveGame`)) _array_index (`self.K2_GetActorLocation` _array_element) true)))
    (:`then_1`
      (bind _returnvalue_2 (`GameplayStatics.SaveGameToSlot` _returnvalue "Default"))
      (return _returnvalue_2))))

(fn `UserConstructionScript`)