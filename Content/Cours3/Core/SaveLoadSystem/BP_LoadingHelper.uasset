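; BP_LoadingHelper is an actor that shows a loading screen and requests streamed levels when play begins.
; It adds WBP_Loading to the viewport, then after a short delay calls a non-blocking stream load on each LevelsToLoad entry.
; Load completion, wired inside the loop rather than after it, moves the player to the GameInstance's spawn position, removes the screen and calls CallOnFinishedLoading on the main game mode.
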(event `self.ReceiveBeginPlay`
  (set `self.MaimGameMode` (`/Game/Cours3/Core/BPFL_MainGame.GetMainGameMode`))
  (`|ExecutionSequence`
    (:`then_0`
      (bind _returnvalue (`|CreateWidget` "/Game/Cours3/UI/WBP_Loading.WBP_Loading_C" (`GameplayStatics.GetPlayerController` 0)))
      (`UserWidget.AddToViewport` _returnvalue 0)
      (set `self.LoadingScreen` _returnvalue))
    (:`then_1`
      (`KismetSystemLibrary.Delay` 0.1)
      (for _array_element (`self.LevelsToLoad`)
        (`GameplayStatics.LoadStreamLevelBySoftObjectPtr` _array_element true)
        (`|ExecutionSequence`
          (:`then_0`
            (bind _asbp_main_gi (cast `/Game/Cours3/Core/BP_MainGI` (`GameplayStatics.GetGameInstance`)))
            (`self.K2_SetActorLocation` (`GameplayStatics.GetPlayerPawn` 0) (`/Game/Cours3/Core/BP_MainGI.PlayerSpawnPosition` _asbp_main_gi) false false))
          (:`then_1`
            (`Widget.RemoveFromParent` (`self.LoadingScreen`))
            (`/Game/Cours3/Core/BP_Main_GM.OnFinishedLoading` (`self.MaimGameMode`))))))))

(fn `UserConstructionScript`)