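; Construction script example actor that lines a spline with half-scale static mesh platforms.
; The construction script divides the spline length by PlatformDistance and adds a mesh component at each interval in local space.
; BeginPlay spawns another actor of this same class with a health PotionType, so each copy spawns again.
; Disconnected leftover nodes cover sphere scaling from potion size and spline mesh start/end setup.
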(event `self.ReceiveBeginPlay`
  (`|SpawnActorFromClass` "Bp_ConstructionScriptEx_C" (`KismetMathLibrary.MakeTransform` (0.0 0.0 0.0)) "Undefined" "OverrideRootScale" null 14 "/Game/Cours3/Gameplay/Potions/Potion_Health2.Potion_Health2" null))

(fn `UserConstructionScript`
  (locals (NewLocalVar_0 :type Integer :default 0) (NewLocalVar_1 :type "Float (double-precision)" :default 0.0))
  (bind _spline (`self.Spline`))
  (bind _output_get (set `local.NewLocalVar_1` (`SplineComponent.GetDistanceAlongSplineAtSplinePoint` _spline (+ (`SplineComponent.GetNumberOfSplinePoints` _spline) -1))))
  (bind _output_get_2 (set `local.NewLocalVar_0` (`KismetMathLibrary.FTrunc` (/ _output_get (`self.PlatformDistance`)))))
  (for _index (range (+ _output_get_2 1))
    (`AddComponent|NODE_AddStaticMeshComponent-1` :`RelativeTransform` (`KismetMathLibrary.MakeTransform` (`SplineComponent.GetLocationAtDistanceAlongSpline` (`self.Spline`) (* _index (`self.PlatformDistance`)) "Local") (struct) (0.5 0.5 0.5)))))